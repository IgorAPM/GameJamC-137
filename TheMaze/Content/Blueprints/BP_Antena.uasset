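; BP_Antena is an antenna actor that players nudge with the keyboard and that detects other antennas in front of it.
; Enter and Right Shift move it in opposite fixed steps along world Y, measured from its Cone component's location.
; While IsActive, Tick runs a debug-drawn visibility trace along its Arrow.
; The first hit on another BP_Antena sets this actor's rotation through a DoOnce that is never reset.
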(event `self.ReceiveBeginPlay`
  (`self.EnableInput` (`GameplayStatics.GetPlayerController` 0)))

(event `Key|Enter`
  (params (Key :type "Key Structure"))
  (:`Pressed`
    (`self.MoveUP`)))

(event `Key|RightShift`
  (params (Key :type "Key Structure"))
  (:`Pressed`
    (`self.MoveDown`)))

(event `self.ReceiveTick`
  (params (DeltaSeconds :type "Float (single-precision)"))
  (bind _returnvalue (`SceneComponent.K2_GetComponentLocation` (`self.DefaultSceneRoot`)))
  (if (`self.IsActive`)
    (bind (_outhit _returnvalue_2) (`KismetSystemLibrary.LineTraceSingle` :`Start` _returnvalue :`End` (+ _returnvalue (* (`SceneComponent.GetForwardVector` (`self.Arrow`)) 700.0)) :`TraceChannel` "TraceTypeQuery1" :`DrawDebugType` "ForOneFrame"))
    (cast `/Game/Blueprints/BP_Antena` (`.HitActor` (`GameplayStatics.BreakHitResult` _outhit)))
    (`/Engine/EditorBlueprintResources/StandardMacros.DoOnce` false
      (:`Completed`
        (if _returnvalue_2
          (`self.K2_SetActorRotation` (struct :`Pitch` -90.0))
          (else
            (`self.K2_SetActorRotation` (struct))))))))

(fn `MoveDown`
  (bind (_returnvalue_x _returnvalue_y _returnvalue_z) (`KismetMathLibrary.BreakVector` (`SceneComponent.K2_GetComponentLocation` (`self.Cone`))))
  (`self.K2_SetActorLocation` (`KismetMathLibrary.MakeVector` _returnvalue_x (+ _returnvalue_y 50.0) _returnvalue_z)))

(fn `MoveUP`
  (bind (_returnvalue_x _returnvalue_y _returnvalue_z) (`KismetMathLibrary.BreakVector` (`SceneComponent.K2_GetComponentLocation` (`self.Cone`))))
  (`self.K2_SetActorLocation` (`KismetMathLibrary.MakeVector` _returnvalue_x (+ _returnvalue_y -50.0) _returnvalue_z)))

(fn `UserConstructionScript`)