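; BP_KeyPad is a keypad actor that shows a UI_PassKeyPAD widget while a FirstPersonCharacter is inside its Box trigger.
; BeginPlay creates the widget collapsed in the viewport and prints SenhaLevel; Box overlap begin and end toggle its visibility.
; Tick rebinds the widget's Enter and Sair (exit) buttons every frame.
; Sair collapses the pad, while Enter is an empty handler, so this file performs no password check.
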(event `self.ReceiveBeginPlay`
  (bind _returnvalue (`|CreateWidget` "/Game/UI/UI_PassKeyPAD.UI_PassKeyPAD_C"))
  (bind _output_get (set `self.Pad` _returnvalue))
  (`UserWidget.AddToViewport` _output_get 0)
  (`Widget.SetVisibility` _output_get "Collapsed")
  (`KismetSystemLibrary.PrintString` (`self.SenhaLevel`)))

(event `self.Box.OnComponentBeginOverlap`
  (params (OverlappedComponent :type "PrimitiveComponent Object Reference") (OtherActor :type "Actor Object Reference") (OtherComp :type "PrimitiveComponent Object Reference") (OtherBodyIndex :type Integer) (bFromSweep :type Boolean) (SweepResult :type "HitResult Structure (by ref)"))
  (cast `/Game/FirstPersonBP/Blueprints/FirstPersonCharacter` OtherActor)
  (`Widget.SetVisibility` (`self.Pad`) "Visible"))

(event `self.Box.OnComponentEndOverlap`
  (params (OverlappedComponent :type "PrimitiveComponent Object Reference") (OtherActor :type "Actor Object Reference") (OtherComp :type "PrimitiveComponent Object Reference") (OtherBodyIndex :type Integer))
  (cast `/Game/FirstPersonBP/Blueprints/FirstPersonCharacter` OtherActor)
  (`Widget.SetVisibility` (`self.Pad`) "Collapsed"))

(event `self.ReceiveTick`
  (params (DeltaSeconds :type "Float (single-precision)"))
  (bind _pad (`self.Pad`))
  (`|ExecutionSequence`
    (:`then_0`
      (add `/Game/UI/UI_PassKeyPAD.EnterButton` _pad (delegate `Enter`)))
    (:`then_1`
      (add `/Game/UI/UI_PassKeyPAD.SairButton` _pad (delegate `Sair`)))))

(event `Enter`)

(event `Sair`
  (`Widget.SetVisibility` (`self.Pad`) "Collapsed"))

(fn `UserConstructionScript`)