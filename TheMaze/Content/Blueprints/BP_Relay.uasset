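; BP_Relay is a challenge terminal with a random ID and a spotlight colored by difficulty.
; BeginPlay creates the interact prompt and challenge widget, filling the latter with the ID, question and answers.
; While the Stop flag is true, player overlap shows the prompt, then after a delay the challenge.
; The widget's button event, rebound every Tick, removes it after a delay and clears Stop, blocking repeats.
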(event `self.ReceiveBeginPlay`
  (bind _returnvalue (`GameplayStatics.GetPlayerController` 0))
  (bind _wid (`self.Wid`))
  (`|ExecutionSequence`
    (:`then_0`
      (bind _returnvalue_2 (`|CreateWidget` "/Game/UI/DesafiosFaceis/UI_ChalengFacil.UI_ChalengFacil_C"))
      (bind _output_get (set `self.Wid` _returnvalue_2))
      (`UserWidget.AddToViewport` _output_get 0)
      (`Widget.SetVisibility` (`self.Wid`) "Collapsed")
      (`WidgetComponent.SetWidget` (`self.Widget`) _wid)
      (bind _returnvalue_3 (`|CreateWidget` "/Game/UI/UI_Interact.UI_Interact_C"))
      (bind _output_get_2 (set `self.Interact` _returnvalue_3))
      (`UserWidget.AddToViewport` _output_get_2 0)
      (`Widget.SetVisibility` _output_get_2 "Collapsed")
      (set `/Game/UI/DesafiosFaceis/UI_ChalengFacil.Num` (`KismetStringLibrary.Conv_IntToString` (`self.ComputerID`)) _wid)
      (set `/Game/UI/DesafiosFaceis/UI_ChalengFacil.QuestionString` (`self.ChallengeText`) _wid)
      (set `/Game/UI/DesafiosFaceis/UI_ChalengFacil.AnswersText` (`self.Answers`) _wid)
      (set `/Game/UI/DesafiosFaceis/UI_ChalengFacil.RightArray` (`self.Questions`) _wid))
    (:`then_1`
      (`WidgetBlueprintLibrary.SetInputMode_GameAndUIEx` _returnvalue (`WidgetComponent.GetUserWidgetObject` (`self.Widget`)))
      (set `PlayerController.bShowMouseCursor` true _returnvalue)
      (`SceneComponent.SetVisibility` (`self.Widget`) false false))
    (:`then_2`
      (`self.EnableInput` _returnvalue))))

(event `self.Box.OnComponentBeginOverlap`
  (params (OverlappedComponent :type "PrimitiveComponent Object Reference") (OtherActor :type "Actor Object Reference") (OtherComp :type "PrimitiveComponent Object Reference") (OtherBodyIndex :type Integer) (bFromSweep :type Boolean) (SweepResult :type "HitResult Structure (by ref)"))
  (cast `/Game/FirstPersonBP/Blueprints/FirstPersonCharacter` OtherActor)
  (if (`self.Stop`)
    (`Widget.SetVisibility` (`self.Interact`) "Visible")
    (`KismetSystemLibrary.Delay` 2.0)
    (`SceneComponent.SetVisibility` (`self.Widget`) true false)
    (`Widget.SetVisibility` (`self.Wid`) "Visible")
    (`Widget.SetVisibility` (`self.Interact`) "Collapsed")))

(event `self.ReceiveTick`
  (params (DeltaSeconds :type "Float (single-precision)"))
  (add `/Game/UI/DesafiosFaceis/UI_ChalengFacil.ButtonPressed` (`self.Wid`) (delegate `DestroyWidget`)))

(event `DestroyWidget`
  (`KismetSystemLibrary.Delay` 1.5)
  (`Widget.RemoveFromParent` (`self.Wid`))
  (set `self.Stop` false))

(event `self.Box.OnComponentEndOverlap`
  (params (OverlappedComponent :type "PrimitiveComponent Object Reference") (OtherActor :type "Actor Object Reference") (OtherComp :type "PrimitiveComponent Object Reference") (OtherBodyIndex :type Integer))
  (cast `/Game/FirstPersonBP/Blueprints/FirstPersonCharacter` OtherActor))

(fn `UserConstructionScript`
  (bind _spotlight (`self.SpotLight`))
  (set `self.ComputerID` (`KismetMathLibrary.RandomIntegerInRange` 0 9))
  (switch `/Game/Blueprints/EN_Difficulty` (`self.DifficultySetting`)
    (:`NewEnumerator0`
      (`LightComponent.SetLightColor` _spotlight (struct :`G` 0.682292 :`B` 0.211241 :`A` 1.0) true))
    (:`NewEnumerator1`
      (`LightComponent.SetLightColor` _spotlight (struct :`R` 1.0 :`G` 0.972589 :`A` 1.0) true))
    (:`NewEnumerator2`
      (`LightComponent.SetLightColor` _spotlight (struct :`R` 1.0 :`A` 1.0) true))))